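; BPC_Damagable is a combat component that gives its owning actor health, hit reactions, death, a melee attack and a lobbed throw.
; AttackTrace sphere-traces forward and passes damage to the target's BPC_Damagable through HitReact.
; HitReact plays a montage until health drops below zero, then calls BP_ThirdPersonCharacter's Death or destroys other owners after a delay.
; ThrowLob spawns BP_LobProjectile at the right hand and impulses it toward player 0 using FindVelocity's distance-based arc.
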(event Custom|AttackTrace
  (params (Damage :type Float%20%28double-precision%29))
  (bind (_outhit _hit_) (CallFunction|SphereTraceForward (Components|GetOwner) 1.5e+02 25.0))
  (if _hit_
    (CallFunction|HitReact (Actor|GetComponentbyClass (.HitActor (Collision|BreakHitResult _outhit)) "BPC_Damagable_C") Damage)))

(event Custom|ThrowLob
  (bind _returnvalue (Components|GetOwner))
  (bind _returnvalue_2 (Actor|GetComponentbyClass _returnvalue "/Script/Engine.SkeletalMeshComponent"))
  (bind _returnvalue_3 (Transformation|GetSocketTransform _returnvalue_2 "HandGrip_R" "RTS_World"))
  (bind _returnvalue_4 (Game|SpawnActorfromClass "/Game/Blueprints/Combat/Enemies/BP_LobProjectile.BP_LobProjectile_C" (Math|Transform|MakeTransform (.location _returnvalue_3) (.rotation _returnvalue_3) "0.100000,0.100000,0.100000") "AdjustIfPossibleButAlwaysSpawn" "MultiplyWithRoot" 0 0))
  (bind _output_get (Variables|Default|SetProjectileRef _returnvalue_4))
  (Collision|SetCollisionEnabled (Variables|/Game/Blueprints/Combat/Enemies/BP_LobProjectile.BP_LobProjectile_C|GetCollision _output_get) "QueryAndPhysics")
  (Collision|SetCollisionEnabled (Variables|/Game/Blueprints/Combat/Enemies/BP_LobProjectile.BP_LobProjectile_C|GetProjectile _output_get) "QueryAndPhysics")
  (Utilities|FlowControl|Delay 0.0)
  (Physics|AddImpulse (Variables|/Game/Blueprints/Combat/Enemies/BP_LobProjectile.BP_LobProjectile_C|GetCollision _output_get) (CallFunction|FindVelocity _output_get) "None" true))

(event Custom|Death
  (Utilities|FlowControl|Delay 1.5)
  (Actor|DestroyActor (Components|GetOwner)))

(event Custom|HitReact
  (params (DamageTaken :type Float%20%28double-precision%29))
  (bind _output_get (Variables|Default|SetHealth (- (Variables|Default|GetHealth) DamageTaken)))
  (if (>= _output_get 0.0)
    (Animation|Montage|PlayMontage (Actor|GetComponentbyClass (Components|GetOwner) "/Script/Engine.SkeletalMeshComponent") (Variables|Default|GetHitReactAnim))
    (else
      (bind _asbp_third_person_character (Utilities|Casting|CastToBP_ThirdPersonCharacter (Components|GetOwner))
        (:then
          (Default|Death _asbp_third_person_character))
        (:CastFailed
          (CallFunction|Death))))))

(fn FindVelocity
  (params (Projectile :type Actor%20Object%20Reference))
  (bind _returnvalue (Game|GetPlayerCharacter 0))
  (bind _returnvalue_2 (Transformation|GetActorLocation Projectile))
  (bind _returnvalue_3 (Transformation|GetActorLocation _returnvalue))
  (bind _returnvalue_4 (Math|Vector|GetUnitDirection(Vector) _returnvalue_2 _returnvalue_3))
  (bind _returnvalue_5 (- _returnvalue_2 _returnvalue_3))
  (bind _returnvalue_6 (Math|Vector|VectorLength (Math|Vector|MakeVector (.x _returnvalue_5) (.y _returnvalue_5) 0.0)))
  (bind _returnvalue_7 (/ _returnvalue_6 1e+03))
  (bind _returnvalue_8 (Math|Float|Square _returnvalue_7))
  (bind _returnvalue_9 (* 0.5 -9.8e+02 _returnvalue_8))
  (bind _returnvalue_10 (- _returnvalue_6 _returnvalue_9))
  (bind _returnvalue_11 (/ _returnvalue_10 _returnvalue_7))
  (bind _returnvalue_12 (* _returnvalue_11 (Math|Vector|MakeVector (.x _returnvalue_4) (.y _returnvalue_4) 0.0)))
  (return (Math|Vector|MakeVector (.x _returnvalue_12) (.y _returnvalue_12) (* _returnvalue_7 -1.0 -9.8e+02 0.25))))