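; BP_LobProjectile is an enemy lobbed projectile that damages on impact, either directly or through an area of effect.
; A collision hit on an actor with BPC_Damagable calls its HitReact and destroys the projectile immediately.
; Any other hit queries the AOE overlaps, where a DoOnce limits the weaker HitReact to the first overlapping actor without a validity check, then destroys the projectile after a short delay.
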(event OnComponentHit(Collision)
  (params (HitComponent :type Primitive%20Component%20Object%20Reference) (OtherActor :type Actor%20Object%20Reference) (OtherComp :type Primitive%20Component%20Object%20Reference) (NormalImpulse :type Vector :default "0, 0, 0") (Hit :type Hit%20Result%20Structure%20%28by%20ref%29))
  (bind _returnvalue (Actor|GetComponentbyClass OtherActor "/Game/Blueprints/Combat/BPC_Damagable.BPC_Damagable_C"))
  (Utilities|IsValid _returnvalue
    (:Is%20Valid
      (Default|HitReact _returnvalue 6.0)
      (Actor|DestroyActor))
    (:Is%20Not%20Valid
      (for _array_element (Collision|GetOverlappingActors (Variables|Default|GetAOE) 0 :!class /Script/Engine.PrimitiveComponent)
        (Utilities|FlowControl|DoOnce false
          (:Completed
            (Default|HitReact (Actor|GetComponentbyClass _array_element "/Game/Blueprints/Combat/BPC_Damagable.BPC_Damagable_C") 3.0))))
      (Utilities|FlowControl|Delay 0.2)
      (Actor|DestroyActor))))

(fn ConstructionScript
  (Collision|SetCollisionEnabled (Variables|Default|GetCollision) "QueryAndPhysics"))