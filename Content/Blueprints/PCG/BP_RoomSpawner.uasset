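; BP_RoomSpawner procedurally builds a five-wide grid of rooms at BeginPlay, flagging two as reward rooms.
; Self-calling events spawn BP_MasterRoom actors, set doors and blocks with delays between rooms, add a boss room, then spawn random layouts across the grid.
; The GameInstance save restores the player's death room, removing it from the door pass, and reuses its number as a reward slot if its type matches.
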(event Custom|SpawnRooms
  (bind _returnvalue (Game|SpawnActorfromClass "/Game/Blueprints/PCG/Rooms/BP_MasterRoom.BP_MasterRoom_C" (CallFunction|FindRoomTransform) "Undefined" "MultiplyWithRoot" 0 0))
  (Variables|/Game/Blueprints/PCG/Rooms/BP_MasterRoom.BP_MasterRoom_C|SetRoomNum _returnvalue (Variables|Default|GetCurrRoom))
  (bind _output_get (Variables|/Game/Blueprints/PCG/Rooms/BP_MasterRoom.BP_MasterRoom_C|SetReward? _returnvalue (or (== (Variables|Default|GetCurrRoom) (Variables|Default|GetReward1)) (== (Variables|Default|GetCurrRoom) (Variables|Default|GetReward2)))))
  (Variables|/Game/Blueprints/PCG/Rooms/BP_MasterRoom.BP_MasterRoom_C|SetRoomType _returnvalue (select _output_get "NewEnumerator4" "NewEnumerator0"))
  (Default|BlockOuterExits _returnvalue)
  (Utilities|Array|AddUnique (Variables|Default|GetRooms) _returnvalue)
  (bind _result (Math|Integer|IncrementInt (Variables|Default|GetCurrRoom))
    (:%20%20
      (if (!= _result (+ (Variables|Default|GetRoomAmount) 1))
        (CallFunction|SpawnRooms)
        (else
          (Utilities|FlowControl|Delay 0.2)
          (CallFunction|SetSaveRoom)
          (Variables|Default|SetCurrRoom 0)
          (CallFunction|SpawnBlocksandDoors))))))

(event Custom|SpawnBlocksAndDoors
  (if (!= (+ (Variables|Default|GetCurrRoom) 1) (Variables|Default|GetRoomAmount))
    (Default|DoorsandBlocks (Utilities|Array|Get(acopy) (Variables|Default|GetRooms) (Variables|Default|GetCurrRoom)))
    (Math|Integer|IncrementInt (Variables|Default|GetCurrRoom)
      (:%20%20
        (Utilities|FlowControl|Delay 1.0)
        (Development|PrintString (Utilities|String|ToString(Integer) (Variables|Default|GetCurrRoom)))
        (CallFunction|SpawnBlocksandDoors)))
    (else
      (Game|SpawnActorfromClass "/Game/Blueprints/PCG/Rooms/BP_BossRoom.BP_BossRoom_C" (Math|Transform|MakeTransform (+ (Transformation|GetActorLocation) "10000.000000,0.000000,0.000000") "0, 0, 0" "1.000000,1.000000,1.000000") "Undefined" "MultiplyWithRoot" 0 0)
      (Variables|Default|SetCurrRoom 0)
      (CallFunction|ChooseLayouts))))

(event Custom|ChooseLayouts
  (Game|SpawnActorfromClass (.OutItem (Utilities|Array|Random (Variables|Default|GetLayouts))) (CallFunction|FindRoomTransform) "Undefined" "MultiplyWithRoot" 0 0)
  (bind _result (Math|Integer|IncrementInt (Variables|Default|GetCurrRoom))
    (:%20%20
      (if (!= _result (+ (Variables|Default|GetRoomAmount) 1))
        (CallFunction|ChooseLayouts)))))

(event EventBeginPlay
  (bind _asgi_gjf2025 (Utilities|Casting|CastToGI_GJF2025 (Game|GetGameInstance))
    (:then
      (Variables|Default|SetSave%20Ref (Variables|/Game/Blueprints/SaveSystem/GI_GJF2025.GI_GJF2025_C|GetSaveRef _asgi_gjf2025))
      (CallFunction|SetRewards)
      (CallFunction|SpawnRooms))
    (:CastFailed
      (Development|PrintString "Save Cast Failed (Spawner)"))))

(fn ConstructionScript)

(fn FindRoomTransform
  (bind _currroom (Variables|Default|GetCurrRoom))
  (return (Math|Transform|MakeTransform (+ (Math|Vector|MakeVector (Math|Conversions|ToFloat(Integer) (* (/ (- _currroom 1) 5) 2000)) (Math|Conversions|ToFloat(Integer) (* (- (Math|Integer|%(Integer) (- _currroom 1) 5) 2) 2000)) 0.0) (Transformation|GetActorLocation)))))

(fn SetRewards
  (bind _roomamount (Variables|Default|GetRoomAmount))
  (bind _roomamount_2 (Variables|Default|GetRoomAmount))
  (bind _returnvalue (Math|Random|RandomIntegerinRange 1 _roomamount_2))
  (bind _returnvalue_2 (Math|Random|RandomIntegerinRange 1 _roomamount))
  (if (Utilities|Enum|Equal(Enum) (.roomtype (Variables|/Game/Blueprints/SaveSystem/SG_RunInfo.SG_RunInfo_C|GetDeathRoomInfo (Variables|Default|GetSave%20Ref))) "NewEnumerator4")
    (Variables|Default|SetReward1 (Variables|/Game/Blueprints/SaveSystem/SG_RunInfo.SG_RunInfo_C|GetDeathRoomNum (Variables|Default|GetSave%20Ref)))
    (else
      (Variables|Default|SetReward1 (Math|Integer|SelectInt _returnvalue 19 (and (!= _returnvalue 3) (!= _returnvalue 23))))))
  (Variables|Default|SetReward2 (Math|Integer|SelectInt _returnvalue_2 11 (Math|Boolean|ANDBoolean (!= _returnvalue_2 3) (!= _returnvalue_2 23) (!= _returnvalue_2 (Variables|Default|GetReward1))))))

(fn SetSaveRoom
  (bind _save_ref (Variables|Default|GetSave%20Ref))
  (bind _rooms (Variables|Default|GetRooms))
  (bind _deathroomnum (Variables|/Game/Blueprints/SaveSystem/SG_RunInfo.SG_RunInfo_C|GetDeathRoomNum _save_ref))
  (bind _returnvalue (- _deathroomnum 1))
  (if (> _deathroomnum 0)
    (Default|SpawnSavedRoom (Utilities|Array|Get(acopy) _rooms _returnvalue))
    (Utilities|Array|RemoveIndex _rooms _returnvalue)))