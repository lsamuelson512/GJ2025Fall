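; GI_GJF2025 is the game instance that owns the run info save object and persists it to a single save slot.
; On Init it loads the existing slot and casts it to SG_RunInfo, or creates and immediately saves a new one if none exists.
; It keeps the object in SaveRef, and a SaveGame event writes that reference back to the same slot.
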(event Custom|SaveGame
  (SaveGame|SaveGametoSlot (Variables|Default|GetSaveRef) "Slot1"))

(event EventInit
  (bind _returnvalue (SaveGame|DoesSaveGameExist "Slot1"))
  (if _returnvalue
    (bind _returnvalue_2 (SaveGame|LoadGamefromSlot "Slot1"))
    (bind _assg_run_info (Utilities|Casting|CastToSG_RunInfo _returnvalue_2)
      (:then
        (Variables|Default|SetSaveRef _assg_run_info))
      (:CastFailed
        (Development|PrintString "Save Cast Failed (Game Instance)")))
    (else
      (bind _returnvalue_3 (SaveGame|CreateSaveGameObject "/Game/Blueprints/SaveSystem/SG_RunInfo.SG_RunInfo_C"))
      (bind _output_get (Variables|Default|SetSaveRef _returnvalue_3))
      (SaveGame|SaveGametoSlot _output_get "Slot1"))))