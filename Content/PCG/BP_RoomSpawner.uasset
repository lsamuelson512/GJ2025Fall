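; BP_RoomSpawner is an actor that generates a grid of BP_MasterRoom actors around its location on BeginPlay.
; SpawnRooms calls itself recursively until the room count is reached, numbering and storing each room and calling its BlockOuterExits.
; FindRoomTransform derives each position from the current index, five rooms per row centered on Y, rows advancing along X at fixed spacing.
; The final loop over stored rooms is empty.
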(event Custom|SpawnRooms
  (bind _returnvalue (Game|SpawnActorfromClass "/Game/PCG/Rooms/BP_MasterRoom.BP_MasterRoom_C" (CallFunction|FindRoomTransform) "Undefined" "MultiplyWithRoot" 0 0))
  (Variables|/Game/PCG/Rooms/BP_MasterRoom.BP_MasterRoom_C|SetRoomNum _returnvalue (Variables|Default|GetCurrRoom))
  (Default|BlockOuterExits _returnvalue)
  (Utilities|Array|Add (Variables|Default|GetRooms) _returnvalue)
  (bind _result (Math|Integer|IncrementInt (Variables|Default|GetCurrRoom))
    (:%20%20
      (if (!= _result (+ (Variables|Default|GetRoomAmount) 1))
        (CallFunction|SpawnRooms)
        (else
          (for _array_element (Variables|Default|GetRooms)
            _))))))

(event EventBeginPlay
  (CallFunction|SpawnRooms))

(fn ConstructionScript)

(fn FindRoomTransform
  (bind _currroom (Variables|Default|GetCurrRoom))
  (return (Math|Transform|MakeTransform (+ (Math|Vector|MakeVector (Math|Conversions|ToFloat(Integer) (* (/ (- _currroom 1) 5) 2000)) (Math|Conversions|ToFloat(Integer) (* (- (Math|Integer|%(Integer) (- _currroom 1) 5) 2) 2000)) 0.0) (Transformation|GetActorLocation)))))